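; BP_Light is an interactable light that the player can switch on and off with the F key while nearby.
; Overlapping its Sphere with BP_ThirdPersonCharacter enables input on the actor for that character's player controller, and leaving disables it.
; Pressing F toggles the PointLight's visibility, and the IsOn? function reports that visibility as the light's state.
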(event `self.Sphere.OnComponentBeginOverlap`
  (params (OverlappedComponent :type "PrimitiveComponent Object Reference") (OtherActor :type "Actor Object Reference") (OtherComp :type "PrimitiveComponent Object Reference") (OtherBodyIndex :type Integer) (bFromSweep :type Boolean) (SweepResult :type "HitResult Structure (by ref)"))
  ;[1 1 1] karakterim sphere ile çarpışıyorsa etkileyebilir
  (bind _asbp_third_person_character (cast `/Game/ThirdPerson/Blueprints/BP_ThirdPersonCharacter` OtherActor))
  (bind _asplayer_controller (cast `PlayerController` (`Pawn.GetController` _asbp_third_person_character)))
  (`self.EnableInput` _asplayer_controller))

(event `self.Sphere.OnComponentEndOverlap`
  (params (OverlappedComponent :type "PrimitiveComponent Object Reference") (OtherActor :type "Actor Object Reference") (OtherComp :type "PrimitiveComponent Object Reference") (OtherBodyIndex :type Integer))
  ;[1 1 1] karakterim sphere ile çarpışmıyorsas ışığı etkileyemez
  (bind _asbp_third_person_character (cast `/Game/ThirdPerson/Blueprints/BP_ThirdPersonCharacter` OtherActor))
  (bind _asplayer_controller (cast `PlayerController` (`Pawn.GetController` _asbp_third_person_character)))
  (`self.DisableInput` _asplayer_controller))

(event `Key|F`
  (params (Key :type "Key Structure"))
  (:`Pressed`
    (`SceneComponent.ToggleVisibility` (`self.PointLight`) false)))

(fn `IsOn?`
  (returns (ReturnValue :type Boolean))
  ;[1 1 1] ışık açık mı?
  (return (`SceneComponent.bVisible` (`self.PointLight`))))

(fn `UserConstructionScript`)
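; Master quest Blueprint that tracks a quest's active and completed subgoals, hunting counters and running description.
; Completing a subgoal records it, updates its quest widget and the selected journal view, then activates its following goal indices, forming a branching chain.
; AddGoalForIndex creates goal widgets, but recursively auto-completes goals of one type whose object the player already obtained.
; OnGoalCompleted is an empty hook, and NextSubGoal offers linear advancement.
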(event `OnGoalCompleted`
  (params (GoalIndex :type Integer)))

(fn `AddGoalForIndex`
  (params (Index :type Integer))
  (locals (LocalIndex :type Integer))
  (bind _questwidget (`self.QuestWidget`))
  (bind _localindex (`local.LocalIndex`))
  (bind _goalinfo (`self.GoalAtIndex` (`local.LocalIndex`)))
  (bind _goalinfo_2 (`self.GoalAtIndex` _localindex))
  (bind _output_get (set `local.LocalIndex` Index))
  (if (`self.GoalAlreadyFound` _output_get)
    (`KismetArrayLibrary.Array_Add` (`self.CompletedSubGoal`) (make `/Game/My/Blueprints/Quest/Structures/S_CompletedGoals` _localindex _goalinfo_2 true))
    (`self.OnGoalCompleted` (`local.LocalIndex`))
    (for _array_element (`.FollowingSubGoalIndices_31_235E96A64412AEE74EB51EBD53C5A434` (break `/Game/My/Blueprints/Quest/Structures/S_GoalInfo` _goalinfo_2))
      (`self.AddGoalForIndex` _array_element))
    (return)
    (else
      (bind _returnvalue (`KismetArrayLibrary.Array_Add` (`self.CurrentGoalIndices`) (`local.LocalIndex`)))
      (if (> _returnvalue (`KismetArrayLibrary.Array_LastIndex` (`self.CurrentHuntingAmounts`)))
        (`KismetArrayLibrary.Array_Add` (`self.CurrentHuntingAmounts`)))
      (`KismetArrayLibrary.Array_Add` (`self.CurrentGoal`) _goalinfo)
      (bind _returnvalue_2 (`|CreateWidget` "/Game/My/Widget/SubGoalWidget.SubGoalWidget_C" null _goalinfo self (`self.QuestWidget`)))
      (`KismetArrayLibrary.Array_Add` (`/Game/My/Widget/QuestWidget.SubGoalWidget` _questwidget) _returnvalue_2)
      (`PanelWidget.AddChild` (`/Game/My/Widget/QuestWidget.SubGoalBox` _questwidget) _returnvalue_2)
      (return))))

(fn `CompleteSubGoal`
  (params (SubGoalIndex :type Integer))
  (returns (Succes :type Boolean))
  (locals (LocalSubGoalIndex :type Integer) (LocalCompletedGoal :type "/Game/My/Blueprints/Quest/Structures/S_GoalInfo Structure") (LocalSubGoalWidgetIndex :type Integer :default 0))
  (bind _localsubgoalwidgetindex (`local.LocalSubGoalWidgetIndex`))
  (bind _localsubgoalindex (`local.LocalSubGoalIndex`))
  (bind _questwidget (`self.QuestWidget`))
  (bind (_goalid _type _customgoal _goaltext _additionalname _amounttohunt _goalclass _goallocation _useradius _radius _radiuscolor _updatequestdecription_ _updateddescription) (break `/Game/My/Blueprints/Quest/Structures/S_GoalInfo` (`local.LocalCompletedGoal`)))
  (bind _returnvalue (`KismetArrayLibrary.Array_Find` (`self.CurrentGoalIndices`) (`local.LocalSubGoalIndex`)))
  (bind _subgoalwidget (`/Game/My/Widget/QuestWidget.SubGoalWidget` (`self.QuestWidget`)))
  (set `local.LocalSubGoalIndex` SubGoalIndex)
  (if (`KismetArrayLibrary.Array_Contains` (`self.CurrentGoalIndices`) _localsubgoalindex)
    (bind _output_get (set `local.LocalCompletedGoal` (`|GetArrayItem` (`.SubGoals_28_4875E87947882733F13C68BB23BADEBF` (break `/Game/My/Blueprints/Quest/Structures/S_QuestInfo` (`self.QuestInfo`))) (`local.LocalSubGoalIndex`))))
    (`KismetArrayLibrary.Array_Add` (`self.CompletedSubGoal`) (make `/Game/My/Blueprints/Quest/Structures/S_CompletedGoals` _localsubgoalindex _output_get true))
    (if _updatequestdecription_
      (set `self.CurrentDesc` (`|FormatText` "{Current}{Next}" (`self.CurrentDesc`) _updateddescription))
      (if (`self.SelectedInJournal?`)
        (`/Game/My/Widget/QuestJournal.UpdateDescription` (`/Game/My/Widget/MainWidget.QuestJournal` (`/Game/My/Blueprints/Quest/QuestActors/BP_QuestManager.MainWidget` (`self.QuestManager`))))))
    (`KismetArrayLibrary.Array_RemoveItem` (`self.CurrentGoal`) (`local.LocalCompletedGoal`))
    (set `local.LocalSubGoalWidgetIndex` _returnvalue)
    (`KismetArrayLibrary.Array_Remove` (`self.CurrentHuntingAmounts`) _returnvalue)
    (`KismetArrayLibrary.Array_RemoveItem` (`self.CurrentGoalIndices`) (`local.LocalSubGoalIndex`))
    (`Widget.RemoveFromParent` (`|GetArrayItem` _subgoalwidget _localsubgoalwidgetindex))
    (`KismetArrayLibrary.Array_Remove` _subgoalwidget _localsubgoalwidgetindex)
    (`self.OnGoalCompleted` (`local.LocalSubGoalIndex`))
    (for _array_element (`.FollowingSubGoalIndices_31_235E96A64412AEE74EB51EBD53C5A434` (break `/Game/My/Blueprints/Quest/Structures/S_GoalInfo` (`local.LocalCompletedGoal`)))
      (`self.AddGoalForIndex` _array_element))
    (if (`self.SelectedInJournal?`)
      (`/Game/My/Widget/QuestJournal.GenerateSubGoals` (`/Game/My/Widget/MainWidget.QuestJournal` (`/Game/My/Blueprints/Quest/QuestActors/BP_QuestManager.MainWidget` (`self.QuestManager`)))))
    (if (== (`self.SelectedSubGoalIndex`) (`local.LocalSubGoalIndex`))
      (`/Game/My/Widget/QuestWidget.SelectSubGoal` _questwidget (`|GetArrayItem` (`/Game/My/Widget/QuestWidget.SubGoalWidget` _questwidget))))
    (return true)
    (else
      (return false))))

(fn `GoalAlreadyFound`
  (params (Index :type Integer))
  (returns (Out :type Boolean))
  (locals (LocalBool :type Boolean))
  (bind (_goalid _type _customgoal _goaltext _additionalname _amounttohunt _goalclass) (break `/Game/My/Blueprints/Quest/Structures/S_GoalInfo` (`self.GoalAtIndex` Index)))
  (if (`|EnumEquality` _type "NewEnumerator2")
    (for _array_element (`/Game/ThirdPerson/Blueprints/BP_ThirdPersonCharacter.ObtainedObject` (`/Game/My/Blueprints/Quest/QuestActors/BP_QuestManager.ThirdPersonChar` (`self.QuestManager`)))
      (if (== _array_element _goalclass)
        (set `local.LocalBool` true)
        (break)))
    (return (`local.LocalBool`))
    (else
      (return false))))

(fn `GoalAtIndex`
  (params (Index :type Integer))
  (returns (GoalInfo :type "/Game/My/Blueprints/Quest/Structures/S_GoalInfo Structure"))
  (return (`|GetArrayItem` (`.SubGoals_28_4875E87947882733F13C68BB23BADEBF` (break `/Game/My/Blueprints/Quest/Structures/S_QuestInfo` (`self.QuestInfo`))) Index)))

(fn `NextSubGoal`
  (returns (`Success?` :type Boolean))
  (locals (NextIndex :type Integer))
  (bind _currentgoalindices (`self.CurrentGoalIndices`))
  (bind _returnvalue (+ (`.MaxValue` (`KismetMathLibrary.MaxOfIntArray` (`self.CurrentGoalIndices`))) 1))
  (if (<= _returnvalue (`KismetArrayLibrary.Array_LastIndex` (`.SubGoals_28_4875E87947882733F13C68BB23BADEBF` (break `/Game/My/Blueprints/Quest/Structures/S_QuestInfo` (`self.QuestInfo`)))))
    (set `local.NextIndex` _returnvalue)
    (`KismetArrayLibrary.Array_Clear` _currentgoalindices)
    (`KismetArrayLibrary.Array_Add` _currentgoalindices (`local.NextIndex`))
    (`self.UpdateSubGoals`)
    (return true)
    (else
      (return false))))

(fn `SelectedInJournal?`
  (returns (`Out?` :type Boolean))
  (bind _selectedquest (`/Game/My/Widget/QuestJournal.SelectedQuest` (`/Game/My/Widget/MainWidget.QuestJournal` (`/Game/My/Blueprints/Quest/QuestActors/BP_QuestManager.MainWidget` (`self.QuestManager`)))))
  (return (and (`KismetSystemLibrary.IsValid` _selectedquest) (== _selectedquest self))))

(fn `SetUpStartingGoals`
  (`KismetArrayLibrary.Array_Clear` (`self.CurrentGoalIndices`))
  (for _array_element (`self.StartingSubGoalIndeces`)
    (`self.AddGoalForIndex` _array_element))
  (`KismetArrayLibrary.Array_Resize` (`self.CurrentHuntingAmounts`) (`KismetArrayLibrary.Array_Length` (`self.CurrentGoalIndices`)))
  (`self.UpdateSubGoals`)
  (set `self.CurrentDesc` (`.Description_32_CF6E2D6D4F5CADEA69709D85FDC53BAB` (break `/Game/My/Blueprints/Quest/Structures/S_QuestInfo` (`self.QuestInfo`))))
  (return))

(fn `UpdateSubGoals`
  ;[1 1 1] current goali en başta boşalttık. sonradan da questin alt görevlerini current goal içerisine currentgoalindicesa göre attık. geçerli değerler bunda
  (`KismetArrayLibrary.Array_Clear` (`self.CurrentGoal`))
  (for _array_element (`self.CurrentGoalIndices`)
    (`KismetArrayLibrary.Array_Add` (`self.CurrentGoal`) (`|GetArrayItem` (`.SubGoals_28_4875E87947882733F13C68BB23BADEBF` (break `/Game/My/Blueprints/Quest/Structures/S_QuestInfo` (`self.QuestInfo`))) _array_element)))
  (return))

(fn `UserConstructionScript`)
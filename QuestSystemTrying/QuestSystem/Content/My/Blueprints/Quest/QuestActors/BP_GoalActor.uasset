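; BP_GoalActor is a quest goal actor that marks a target with either a minimap icon sprite or a colored radius circle.
; The construction script uses Useradius to pick which sprite is visible, scales the circle from Radius and tints it with CircleColor.
; On BeginPlay it makes the player character its owner and sets owner-no-see on both sprites, intended to keep them out of the in-game view.
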(event `self.ReceiveBeginPlay`
  ;[1 1 1] minimap üzerindeki hedef ikonunun oyunda gösterilmemesi
  (`self.SetOwner` (`GameplayStatics.GetPlayerCharacter` 0))
  (`PrimitiveComponent.SetOwnerNoSee` (`self.MinimapIcon`) true)
  (`PrimitiveComponent.SetOwnerNoSee` (`self.MinimapRadius`) true))

(fn `UserConstructionScript`
  (bind _minimapradius (`self.MinimapRadius`))
  (bind _useradius_ (`self.useradius?`))
  (bind _radius (`self.radius`))
  (bind _returnvalue (/ _radius 500.0))
  (`SceneComponent.SetVisibility` (`self.MinimapIcon`) (not _useradius_) false)
  (`SceneComponent.SetRelativeScale3D` _minimapradius (`KismetMathLibrary.MakeVector` _returnvalue _radius _returnvalue))
  (`SceneComponent.SetVisibility` _minimapradius _useradius_ false)
  (`PaperSpriteComponent.SetSpriteColor` _minimapradius (`self.CircleColor`)))
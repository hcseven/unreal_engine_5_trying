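; BP_BaseQuests is a base quest Blueprint in the quest system, built around a root objective collection.
; On BeginPlay it creates and stores the root collection, passes it to PopulateObjectives, then activates it.
; The construction and population functions are empty stubs, apparently left for child quests to override.
; A getter exposes the root collection.
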(event `self.ReceiveBeginPlay`
  (bind _rootobjectcollection (`self.ConstructionRootObjectCollection`))
  (bind _output_get (set `self.RootObjectCollection` _rootobjectcollection))
  (`self.PopulateObjectives` _output_get)
  (`/Game/QuestSystem/Objectives/BP_BaseObjective.ActivateObjective` (`self.RootObjectCollection`)))

(fn `ConstructionRootObjectCollection`
  (returns (RootObjectCollection :type "/Game/QuestSystem/Objectives/BP_ObjCollection Object Reference"))
  (return null))

(fn `GetRootObjectiveCollection`
  (returns (RootObject :type "/Game/QuestSystem/Objectives/BP_ObjCollection Object Reference"))
  (return (`self.RootObjectCollection`)))

(fn `PopulateObjectives`
  (params (RootObjectCollection :type "/Game/QuestSystem/Objectives/BP_ObjCollection Object Reference"))
  (return))

(fn `UserConstructionScript`)
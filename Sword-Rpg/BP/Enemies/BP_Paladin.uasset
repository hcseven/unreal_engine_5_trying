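; BP_Paladin is an enemy character Blueprint for a paladin equipped with a sword and shield.
; Its construction script attaches the shield and sword to left and right hand sockets on the mesh, keeping relative transforms, then calls the parent construction script.
; The sword is set to query-and-probe collision that overlaps all channels.
; The event graph holds only disabled placeholder events, with no active logic.
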(fn `UserConstructionScript`
  (bind _sword (`self.sword`))
  (bind _mesh (`self.Mesh`))
  (`SceneComponent.K2_AttachToComponent` (`self.shield`) _mesh "Socket_LeftHand" "KeepRelative" "KeepRelative" "KeepRelative" true)
  (`PrimitiveComponent.SetCollisionEnabled` _sword "QueryAndProbe")
  (`PrimitiveComponent.SetCollisionResponseToAllChannels` _sword "ECR_Overlap")
  (`SceneComponent.K2_AttachToComponent` _sword _mesh "Socket_RightHand" "KeepRelative" "KeepRelative" "KeepRelative" true)
  (`parent.UserConstructionScript`))